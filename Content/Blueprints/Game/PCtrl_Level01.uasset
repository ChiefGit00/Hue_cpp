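; Player controller for Level 01 that manages the HUD and the end-of-level screens.
; SetUI creates and shows a given widget with mouse cursor, permanent capture and touch interface.
; LevelFinish and LifeOver pause the game and swap that widget for the finish or game-over screen.
; On finish, it first saves the score under the current level name through BP_GameInstance.
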(event Custom|LevelFinish
  (Game|SetGamePaused true)
  (Widget|RemovefromParent (stale Custom|SetUI _returnvalue))
  (bind _asbp_game_instance (Utilities|Casting|CastToBP_GameInstance (Game|GetGameInstance)))
  (bind _returnvalue (Game|GetCurrentLevelName true))
  (Default|SaveLevelScore _asbp_game_instance (Utilities|String|StringToName _returnvalue) (Variables|Default|GetScore))
  (bind _returnvalue_2 (UserInterface|CreateWidget "/Game/UI/UI_Finish.UI_Finish_C"))
  (UserInterface|Viewport|AddtoViewport _returnvalue_2 0)
  (Variables|Default|SetbShowMouseCursor true))

(event Custom|LifeOver
  (Game|SetGamePaused true)
  (Widget|RemovefromParent (stale Custom|SetUI _returnvalue))
  (bind _returnvalue (UserInterface|CreateWidget "/Game/UI/UI_Over.UI_Over_C"))
  (UserInterface|Viewport|AddtoViewport _returnvalue 0)
  (Variables|Default|SetbShowMouseCursor true))

(event Custom|SetUI
  (params (Widget :type User%20Widget%20Class%20Reference))
  (bind _returnvalue (UserInterface|CreateWidget Widget))
  (UserInterface|Viewport|AddtoViewport _returnvalue 0)
  (Class|GameplayStatics|SetViewportMouseCaptureMode "CapturePermanently")
  (Variables|Default|SetbShowMouseCursor true)
  (Class|PlayerController|ActivateTouchInterface))

(fn ConstructionScript)