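; Runner player pawn that constantly moves along +X, sidesteps along Y and collects colour-matched coins and health pickups.
; Timelines drive sidesteps with fold animations; Jump input instantly raises the pawn.
; Outside sidesteps, a downward trace finding no ground switches the mesh to physics.
; The laser's colour sets its material and collision and gates coin scoring; Finish and Over report to PCtrl_Level01 after a delay.
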(event OnComponentBeginOverlap(PickUpLaser_0)
  (params (OverlappedComponent :type Primitive%20Component%20Object%20Reference) (OtherActor :type Actor%20Object%20Reference) (OtherComp :type Primitive%20Component%20Object%20Reference) (OtherBodyIndex :type Integer) (bFromSweep :type Boolean) (SweepResult :type Hit%20Result%20Structure%20%28by%20ref%29))
  (bind _asbp_pick_ups (Utilities|Casting|CastToBP_PickUps OtherActor))
  (switch Utilities|FlowControl|Switch|SwitchonE_PickUpTypes (Variables|/Game/Blueprints/Actors/BP_PickUps.BP_PickUps_C|GetType _asbp_pick_ups)
    (:NewEnumerator0
      (bind _asbp_coins (Utilities|Casting|CastToBP_Coins _asbp_pick_ups))
      (if (Utilities|Enum|Equal(Enum) (Variables|/Game/Blueprints/Actors/BP_Coins.BP_Coins_C|GetColour _asbp_coins) (Variables|Default|GetColour_0))
        (Variables|Default|SetScore_0 (+ (Variables|Default|GetScore_0) (Variables|/Game/Blueprints/Actors/BP_PickUps.BP_PickUps_C|GetValue _asbp_coins)))
        (Default|SoundSuccess _asbp_pick_ups :!label _label)
        (if (<= (stale _output_get) 0.0)
          (CallFunction|Over))
        (else
          (Audio|PlaySound2D "/Game/Sound/Invalid.Invalid" 1.0 1.0 0.0 0 0))))
    (:NewEnumerator1
      (bind _output_get (Variables|Default|SetHealth_0 (+ (Variables|Default|GetHealth_0) (Math|Conversions|ToFloat(Integer) (Variables|/Game/Blueprints/Actors/BP_PickUps.BP_PickUps_C|GetValue _asbp_pick_ups)))))
      (Variables|Default|SetHealthPerce_0 (/ _output_get 1e+02))
      (goto _label))))

(event Custom|MoveY
  (params (+ve :type Boolean))
  (bind _returnvalue (Transformation|GetActorLocation))
  (Variables|Default|SetbYAxis_0 +ve)
  (Variables|Default|SetbJump_0 true)
  (if (Variables|Default|GetbMoveY_0)
    (Variables|Default|SetbMoveY_0 false)
    (Variables|Default|SetYAxis_0 (.y _returnvalue))
    (Components|Animation|PlayAnimation (Variables|Default|GetSkeletalMesh_0) "/Game/SkeletalMesh/Player001_Anim_Armature_FoldUp.Player001_Anim_Armature_FoldUp" false)
    (if (Variables|Default|GetbYAxis_0)
      (bind _y_ (Timeline|+300_0 PlayFromStart)
        (:Update
          (Transformation|SetActorLocation (Math|Vector|MakeVector (.x _returnvalue) (+ (Variables|Default|GetYAxis_0) _y_) (.z _returnvalue)) false false))
        (:Finished
          (Variables|Default|SetbMoveY_0 true :!label _label)
          (Variables|Default|SetbJump_0 false)
          (Components|Animation|PlayAnimation (Variables|Default|GetSkeletalMesh_0) "/Game/SkeletalMesh/Player001_Anim_Armature_FoldDown.Player001_Anim_Armature_FoldDown" false)))
      (else
        (bind _y__2 (Timeline|-300_0 PlayFromStart)
          (:Update
            (Transformation|SetActorLocation (Math|Vector|MakeVector (.x _returnvalue) (+ _y__2 (Variables|Default|GetYAxis_0)) (.z _returnvalue)) false false))
          (:Finished
            (goto _label)))))))

(event Custom|Finish
  (bind _ctrl_0 (Variables|Default|GetCtrl_0))
  (Variables|Default|SetbFinish_0 true)
  (Utilities|FlowControl|Delay 0.5)
  (Variables|/Game/Blueprints/Game/PCtrl_Level01.PCtrl_Level01_C|SetScore _ctrl_0 (Variables|Default|GetScore_0))
  (Default|LevelFinish _ctrl_0))

(event Custom|Over
  (Variables|Default|SetbFinish_0 true)
  (Utilities|FlowControl|Delay 0.5)
  (Default|LifeOver (Variables|Default|GetCtrl_0)))

(event EventTick
  (params (DeltaSeconds :type Float%20%28single-precision%29))
  (bind _arrowz_0 (Variables|Default|GetArrowZ_0))
  (bind _skeletalmesh_0 (Variables|Default|GetSkeletalMesh_0))
  (bind _returnvalue (Transformation|GetWorldLocation _arrowz_0))
  (Pawn|Input|AddMovementInput "1.000000, 0,0.000000" (Variables|Default|GetSpeed_0) false)
  (if (not (Variables|Default|GetbJump_0))
    (Utilities|FlowControl|Sequence
      (:then_0
        (bind (_outhit _returnvalue_2) (Collision|LineTraceByChannel _returnvalue (+ _returnvalue "0, 0,-400.000000") "TraceTypeQuery1" false 0 "ForDuration"))
        (if (not _returnvalue_2)
          (Collision|SetCollisionEnabled _skeletalmesh_0 "QueryOnly")
          (Physics|SetSimulatePhysics _skeletalmesh_0 true))))))

(event EventPossessed
  (params (NewController :type Controller%20Object%20Reference))
  (bind _aspctrl_level_01 (Utilities|Casting|CastToPCtrl_Level01 NewController))
  (Variables|Default|SetCtrl_0 _aspctrl_level_01))

(event EventDeath
  (CallFunction|Over))

(event Input|ActionEvents|InputActionJump
  (params (Key :type Key%20Structure :default "None"))
  (bind _returnvalue (Transformation|GetActorLocation))
  (:Pressed
    (Transformation|SetActorLocation (Math|Vector|MakeVector (.x _returnvalue) (.y _returnvalue) (+ (.z _returnvalue) 5e+02)) false false)))

(event Input|AxisEvents|InputAxisMoveSide
  (params (AxisValue :type Float%20%28single-precision%29))
  (bind _returnvalue (Transformation|GetActorLocation))
  (if (> AxisValue 0.0)
    (Variables|Default|SetbYAxis_0 true)
    (Variables|Default|SetbJump_0 true :!label _label)
    (if (Variables|Default|GetbMoveY_0)
      (Variables|Default|SetbMoveY_0 false)
      (Variables|Default|SetYAxis_0 (.y _returnvalue))
      (Components|Animation|PlayAnimation (Variables|Default|GetSkeletalMesh_0) "/Game/SkeletalMesh/Player001_Anim_Armature_FoldUp.Player001_Anim_Armature_FoldUp" false)
      (if (Variables|Default|GetbYAxis_0)
        (bind _y_ (Timeline|+300_0 PlayFromStart)
          (:Update
            (Transformation|SetActorLocation (Math|Vector|MakeVector (.x _returnvalue) (+ (Variables|Default|GetYAxis_0) _y_) (.z _returnvalue)) false false))
          (:Finished
            (Variables|Default|SetbMoveY_0 true :!label _label_2)
            (Variables|Default|SetbJump_0 false)
            (Components|Animation|PlayAnimation (Variables|Default|GetSkeletalMesh_0) "/Game/SkeletalMesh/Player001_Anim_Armature_FoldDown.Player001_Anim_Armature_FoldDown" false)))
        (else
          (bind _y__2 (Timeline|-300_0 PlayFromStart)
            (:Update
              (Transformation|SetActorLocation (Math|Vector|MakeVector (.x _returnvalue) (+ _y__2 (Variables|Default|GetYAxis_0)) (.z _returnvalue)) false false))
            (:Finished
              (goto _label_2))))))
    (elif (< AxisValue 0.0)
      (Variables|Default|SetbYAxis_0 false)
      (goto _label))))

(fn ConstructionScript
  (CallFunction|PickUpColourChange "NewEnumerator3"))

(fn PickUpColourChange
  (params (NewColour :type E_PickUpColours%20Enum :default "NewEnumerator3"))
  (bind _skeletalmesh_0 (Variables|Default|GetSkeletalMesh_0))
  (bind _pickuplaser_0 (Variables|Default|GetPickUpLaser_0))
  (switch Utilities|FlowControl|Switch|SwitchonE_PickUpColours NewColour
    (:NewEnumerator3
      (Rendering|Material|SetMaterial _skeletalmesh_0 3 "/Game/Materials/PickUpLaser/M_LaserNone.M_LaserNone")
      (Collision|SetCollisionEnabled _pickuplaser_0 "NoCollision")
      (Variables|Default|SetColour_0 "NewEnumerator3"))
    (:NewEnumerator0
      (Rendering|Material|SetMaterial _skeletalmesh_0 3 "/Game/Materials/PickUpLaser/M_LaserYellow.M_LaserYellow")
      (Collision|SetCollisionEnabled _pickuplaser_0 "QueryAndPhysics")
      (Variables|Default|SetColour_0 "NewEnumerator0"))
    (:NewEnumerator1
      (Rendering|Material|SetMaterial _skeletalmesh_0 3 "/Game/Materials/PickUpLaser/M_LaserRed.M_LaserRed")
      (Collision|SetCollisionEnabled _pickuplaser_0 "QueryAndPhysics")
      (Variables|Default|SetColour_0 "NewEnumerator1"))
    (:NewEnumerator2
      (Rendering|Material|SetMaterial _skeletalmesh_0 3 "/Game/Materials/PickUpLaser/M_LaserGreen.M_LaserGreen")
      (Collision|SetCollisionEnabled _pickuplaser_0 "QueryAndPhysics")
      (Variables|Default|SetColour_0 "NewEnumerator2"))))