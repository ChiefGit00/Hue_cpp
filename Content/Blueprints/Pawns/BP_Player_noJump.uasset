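; Player pawn for an auto-runner level that constantly moves along +X and collects colour-coded pickups.
; Side input triggers one of two timelines that shift it along Y, with fold animations and a gate against overlapping moves.
; The laser's overlap adds score for colour-matched coins or restores health; PickUpColourChange sets its material, collision and colour.
; Finish and death report to the cached PCtrl_Level01 after a short delay.
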(event OnComponentBeginOverlap(PickUpLaser)
  (params (OverlappedComponent :type Primitive%20Component%20Object%20Reference) (OtherActor :type Actor%20Object%20Reference) (OtherComp :type Primitive%20Component%20Object%20Reference) (OtherBodyIndex :type Integer) (bFromSweep :type Boolean) (SweepResult :type Hit%20Result%20Structure%20%28by%20ref%29))
  (bind _asbp_pick_ups (Utilities|Casting|CastToBP_PickUps OtherActor))
  (switch Utilities|FlowControl|Switch|SwitchonE_PickUpTypes (Variables|/Game/Blueprints/Actors/BP_PickUps.BP_PickUps_C|GetType _asbp_pick_ups)
    (:NewEnumerator0
      (bind _asbp_coins (Utilities|Casting|CastToBP_Coins _asbp_pick_ups))
      (if (Utilities|Enum|Equal(Enum) (Variables|/Game/Blueprints/Actors/BP_Coins.BP_Coins_C|GetColour _asbp_coins) (Variables|Default|GetColour))
        (Variables|Default|SetScore (+ (Variables|Default|GetScore) (Variables|/Game/Blueprints/Actors/BP_PickUps.BP_PickUps_C|GetValue _asbp_coins)))
        (Default|SoundSuccess _asbp_pick_ups :!label _label)
        (if (<= (stale _output_get) 0.0)
          (CallFunction|Over))
        (else
          (Audio|PlaySound2D "/Game/Sound/Invalid.Invalid" 1.0 1.0 0.0 0 0))))
    (:NewEnumerator1
      (bind _output_get (Variables|Default|SetHealth (+ (Variables|Default|GetHealth) (Math|Conversions|ToFloat(Integer) (Variables|/Game/Blueprints/Actors/BP_PickUps.BP_PickUps_C|GetValue _asbp_pick_ups)))))
      (Variables|Default|SetHealthPerce (/ _output_get 1e+02))
      (goto _label))))

(event Custom|MoveY
  (params (+ve :type Boolean))
  (bind _returnvalue (Transformation|GetActorLocation))
  (Variables|Default|SetbYAxis +ve)
  (Variables|Default|SetbJump true)
  (if (Variables|Default|GetbMoveY)
    (Variables|Default|SetbMoveY false)
    (Variables|Default|SetYAxis (.y _returnvalue))
    (Components|Animation|PlayAnimation (Variables|Default|GetSkeletalMesh) "/Game/SkeletalMesh/Player001_Anim_Armature_FoldUp.Player001_Anim_Armature_FoldUp" false)
    (if (Variables|Default|GetbYAxis)
      (bind _y_ (Timeline|+300 PlayFromStart)
        (:Update
          (Transformation|SetActorLocation (Math|Vector|MakeVector (.x _returnvalue) (+ (Variables|Default|GetYAxis) _y_) (.z _returnvalue)) false false))
        (:Finished
          (Variables|Default|SetbMoveY true :!label _label)
          (Variables|Default|SetbJump false)
          (Components|Animation|PlayAnimation (Variables|Default|GetSkeletalMesh) "/Game/SkeletalMesh/Player001_Anim_Armature_FoldDown.Player001_Anim_Armature_FoldDown" false)))
      (else
        (bind _y__2 (Timeline|-300 PlayFromStart)
          (:Update
            (Transformation|SetActorLocation (Math|Vector|MakeVector (.x _returnvalue) (+ _y__2 (Variables|Default|GetYAxis)) (.z _returnvalue)) false false))
          (:Finished
            (goto _label)))))))

(event Custom|Finish
  (bind _ctrl (Variables|Default|GetCtrl))
  (Variables|Default|SetbFinish true)
  (Utilities|FlowControl|Delay 0.5)
  (Variables|/Game/Blueprints/Game/PCtrl_Level01.PCtrl_Level01_C|SetScore _ctrl (Variables|Default|GetScore))
  (Default|LevelFinish _ctrl))

(event Custom|Over
  (Variables|Default|SetbFinish true)
  (Utilities|FlowControl|Delay 0.5)
  (Default|LifeOver (Variables|Default|GetCtrl)))

(event EventTick
  (params (DeltaSeconds :type Float%20%28single-precision%29))
  (Pawn|Input|AddMovementInput "1.000000, 0,0.000000" (Variables|Default|GetSpeed) false))

(event EventPossessed
  (params (NewController :type Controller%20Object%20Reference))
  (bind _aspctrl_level_01 (Utilities|Casting|CastToPCtrl_Level01 NewController))
  (Variables|Default|SetCtrl _aspctrl_level_01))

(event EventDeath
  (CallFunction|Over))

(event Input|AxisEvents|InputAxisMoveSide
  (params (AxisValue :type Float%20%28single-precision%29))
  (bind _returnvalue (Transformation|GetActorLocation))
  (if (> AxisValue 0.0)
    (Variables|Default|SetbYAxis true)
    (Variables|Default|SetbJump true :!label _label)
    (if (Variables|Default|GetbMoveY)
      (Variables|Default|SetbMoveY false)
      (Variables|Default|SetYAxis (.y _returnvalue))
      (Components|Animation|PlayAnimation (Variables|Default|GetSkeletalMesh) "/Game/SkeletalMesh/Player001_Anim_Armature_FoldUp.Player001_Anim_Armature_FoldUp" false)
      (if (Variables|Default|GetbYAxis)
        (bind _y_ (Timeline|+300 PlayFromStart)
          (:Update
            (Transformation|SetActorLocation (Math|Vector|MakeVector (.x _returnvalue) (+ (Variables|Default|GetYAxis) _y_) (.z _returnvalue)) false false))
          (:Finished
            (Variables|Default|SetbMoveY true :!label _label_2)
            (Variables|Default|SetbJump false)
            (Components|Animation|PlayAnimation (Variables|Default|GetSkeletalMesh) "/Game/SkeletalMesh/Player001_Anim_Armature_FoldDown.Player001_Anim_Armature_FoldDown" false)))
        (else
          (bind _y__2 (Timeline|-300 PlayFromStart)
            (:Update
              (Transformation|SetActorLocation (Math|Vector|MakeVector (.x _returnvalue) (+ _y__2 (Variables|Default|GetYAxis)) (.z _returnvalue)) false false))
            (:Finished
              (goto _label_2))))))
    (elif (< AxisValue 0.0)
      (Variables|Default|SetbYAxis false)
      (goto _label))))

(fn ConstructionScript
  (CallFunction|PickUpColourChange "NewEnumerator3"))

(fn PickUpColourChange
  (params (NewColour :type E_PickUpColours%20Enum :default "NewEnumerator3"))
  (bind _skeletalmesh (Variables|Default|GetSkeletalMesh))
  (bind _pickuplaser (Variables|Default|GetPickUpLaser))
  (switch Utilities|FlowControl|Switch|SwitchonE_PickUpColours NewColour
    (:NewEnumerator3
      (Rendering|Material|SetMaterial _skeletalmesh 3 "/Game/Materials/PickUpLaser/M_LaserNone.M_LaserNone")
      (Collision|SetCollisionEnabled _pickuplaser "NoCollision")
      (Variables|Default|SetColour "NewEnumerator3"))
    (:NewEnumerator0
      (Rendering|Material|SetMaterial _skeletalmesh 3 "/Game/Materials/PickUpLaser/M_LaserYellow.M_LaserYellow")
      (Collision|SetCollisionEnabled _pickuplaser "QueryAndPhysics")
      (Variables|Default|SetColour "NewEnumerator0"))
    (:NewEnumerator1
      (Rendering|Material|SetMaterial _skeletalmesh 3 "/Game/Materials/PickUpLaser/M_LaserRed.M_LaserRed")
      (Collision|SetCollisionEnabled _pickuplaser "QueryAndPhysics")
      (Variables|Default|SetColour "NewEnumerator1"))
    (:NewEnumerator2
      (Rendering|Material|SetMaterial _skeletalmesh 3 "/Game/Materials/PickUpLaser/M_LaserGreen.M_LaserGreen")
      (Collision|SetCollisionEnabled _pickuplaser "QueryAndPhysics")
      (Variables|Default|SetColour "NewEnumerator2"))))