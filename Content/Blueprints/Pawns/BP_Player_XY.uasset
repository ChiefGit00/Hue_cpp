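; Player pawn that sidesteps along the world Y axis on MoveSide input or a MoveY event, calling parent Tick logic.
; A gated move plays one of two direction-specific timelines to offset Y, with fold-up and fold-down animations at start and finish.
; Outside moves, Tick traces down from ArrowZ to snap height to the surface below, or sets Zaxis negative when none is found.
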(event EventTick
  (params (DeltaSeconds :type Float%20%28single-precision%29))
  (bind _returnvalue (Transformation|GetActorLocation))
  (bind _arrowz (Variables|Default|GetArrowZ))
  (bind _returnvalue_2 (Transformation|GetWorldLocation _arrowz))
  (|CallParentFunction DeltaSeconds)
  (if (not (Variables|Default|GetbJump))
    (bind (_outhit _returnvalue_3) (Collision|LineTraceByChannel _returnvalue_2 (+ _returnvalue_2 "0, 0,-400.000000") "TraceTypeQuery1" false 0 "None"))
    (if _returnvalue_3
      (Transformation|SetActorLocation (Math|Vector|MakeVector (.x _returnvalue) (.y _returnvalue) (- (.z (.location _outhit)) 1e+01)) false false)
      (else
        (Variables|Default|SetZaxis -1.0)))))

(event EventMoveY
  (params (+ve :type Boolean))
  (bind _returnvalue (Transformation|GetActorLocation))
  (Variables|Default|SetbYAxis +ve)
  (Variables|Default|SetbJump true)
  (if (Variables|Default|GetbMoveY)
    (Variables|Default|SetbMoveY false)
    (Variables|Default|SetYAxis (.y _returnvalue))
    (Components|Animation|PlayAnimation (Variables|Default|GetSkeletalMesh) "/Game/SkeletalMesh/Player001_Anim_Armature_FoldUp.Player001_Anim_Armature_FoldUp" false)
    (if (Variables|Default|GetbYAxis)
      (bind _y_ (Timeline|Timeline_0 PlayFromStart)
        (:Update
          (Transformation|SetActorLocation (Math|Vector|MakeVector (.x _returnvalue) (+ (Variables|Default|GetYAxis) _y_) (.z _returnvalue)) false false))
        (:Finished
          (Variables|Default|SetbMoveY true :!label _label)
          (Variables|Default|SetbJump false)
          (Components|Animation|PlayAnimation (Variables|Default|GetSkeletalMesh) "/Game/SkeletalMesh/Player001_Anim_Armature_FoldDown.Player001_Anim_Armature_FoldDown" false)))
      (else
        (bind _y__2 (Timeline|Timeline_1 PlayFromStart)
          (:Update
            (Transformation|SetActorLocation (Math|Vector|MakeVector (.x _returnvalue) (+ _y__2 (Variables|Default|GetYAxis)) (.z _returnvalue)) false false))
          (:Finished
            (goto _label)))))))

(event Input|AxisEvents|InputAxisMoveSide
  (params (AxisValue :type Float%20%28single-precision%29))
  (bind _returnvalue (Transformation|GetActorLocation))
  (if (> AxisValue 0.0)
    (Variables|Default|SetbYAxis true)
    (Variables|Default|SetbJump true :!label _label)
    (if (Variables|Default|GetbMoveY)
      (Variables|Default|SetbMoveY false)
      (Variables|Default|SetYAxis (.y _returnvalue))
      (Components|Animation|PlayAnimation (Variables|Default|GetSkeletalMesh) "/Game/SkeletalMesh/Player001_Anim_Armature_FoldUp.Player001_Anim_Armature_FoldUp" false)
      (if (Variables|Default|GetbYAxis)
        (bind _y_ (Timeline|Timeline_0 PlayFromStart)
          (:Update
            (Transformation|SetActorLocation (Math|Vector|MakeVector (.x _returnvalue) (+ (Variables|Default|GetYAxis) _y_) (.z _returnvalue)) false false))
          (:Finished
            (Variables|Default|SetbMoveY true :!label _label_2)
            (Variables|Default|SetbJump false)
            (Components|Animation|PlayAnimation (Variables|Default|GetSkeletalMesh) "/Game/SkeletalMesh/Player001_Anim_Armature_FoldDown.Player001_Anim_Armature_FoldDown" false)))
        (else
          (bind _y__2 (Timeline|Timeline_1 PlayFromStart)
            (:Update
              (Transformation|SetActorLocation (Math|Vector|MakeVector (.x _returnvalue) (+ _y__2 (Variables|Default|GetYAxis)) (.z _returnvalue)) false false))
            (:Finished
              (goto _label_2))))))
    (elif (< AxisValue 0.0)
      (Variables|Default|SetbYAxis false)
      (goto _label))))

(fn ConstructionScript
  (|CallParentFunction))