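; BP_PickUps is a pickup actor that disappears when anything overlaps its Box component.
; On overlap it disables the Box's collision to prevent retriggering, hides the StaticMesh, then destroys itself after a short delay.
; A separate SoundSuccess function assigns a sound to PickUpSound and plays it, but nothing in this Blueprint calls it.
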(event OnComponentBeginOverlap(Box)
  (params (OverlappedComponent :type Primitive%20Component%20Object%20Reference) (OtherActor :type Actor%20Object%20Reference) (OtherComp :type Primitive%20Component%20Object%20Reference) (OtherBodyIndex :type Integer) (bFromSweep :type Boolean) (SweepResult :type Hit%20Result%20Structure%20%28by%20ref%29))
  (Collision|SetCollisionEnabled (Variables|Default|GetBox) "NoCollision")
  (Rendering|SetVisibility (Variables|Default|GetStaticMesh) false false)
  (Utilities|FlowControl|Delay 0.5)
  (Actor|DestroyActor))

(event EventBeginPlay)

(event Collision|EventActorBeginOverlap
  (params (OtherActor :type Actor%20Object%20Reference)))

(event EventTick
  (params (DeltaSeconds :type Float%20%28single-precision%29)))

(fn ConstructionScript)

(fn SoundSuccess
  (bind _pickupsound (Variables|Default|GetPickUpSound))
  (Audio|Components|Audio|SetSound _pickupsound (Variables|Default|GetSound))
  (Audio|Components|Audio|Play _pickupsound 0.0))